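; Actor for a character folder, with a randomized portrait and personal record shown on travel and identity papers.
; Construction adds random neck, nose, eye and head sprites; BeginPlay rolls identity, health, background and financial data, then hides the folder.
; Once MouseController reports GameStarted, every Tick refreshes the texts, unhides the folder, plays its flipbook and a timeline sliding it toward EndLocation.
; Both papers appear after a flipbook-length delay.
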(event `self.ReceiveBeginPlay`
  (`self.InitArrays`)
  (`self.InitOthers`)
  (`self.SetActorHiddenInGame` true)
  (`ActorComponent.SetActive` (`self.AnimChemise`) false false)
  (`KismetSystemLibrary.PrintString` (`self.Nom`))
  (`KismetSystemLibrary.PrintString` (`self.GroupeSanguin`))
  (`KismetSystemLibrary.PrintString` (`self.Permis`))
  (`KismetSystemLibrary.PrintString` (`self.Antécédent`))
  (`KismetSystemLibrary.PrintString` (`self.Addiction`))
  (`KismetSystemLibrary.PrintString` (`KismetStringLibrary.Conv_IntToString` (`self.Poids`)))
  (`KismetSystemLibrary.PrintString` (`KismetStringLibrary.Conv_IntToString` (`self.Revenu`)))
  (`KismetSystemLibrary.PrintString` (`KismetStringLibrary.Conv_DoubleToString` (`self.Taille`))))

(event `self.ReceiveTick`
  (params (DeltaSeconds :type "Float (single-precision)"))
  (bind _sex_txt (`self.sex_txt`))
  (bind _animchemise (`self.AnimChemise`))
  (bind _asmouse_controller (cast `/Game/BluePrint/Zawarudo_BPs/MouseController` (`GameplayStatics.GetPlayerController` 0)))
  (if (`/Game/BluePrint/Zawarudo_BPs/MouseController.GameStarted` _asmouse_controller)
    ;[1 1 1] SetAllTextVariable
    (`TextRenderComponent.K2_SetText` (`self.Tete_Pays`) (`KismetTextLibrary.Conv_StringToText` (`self.Pays`)))
    (`TextRenderComponent.K2_SetText` (`self.Groupe_Sanguin`) (`KismetTextLibrary.Conv_StringToText` (`self.GroupeSanguin`)))
    (`TextRenderComponent.K2_SetText` (`self.Antecedent`) (`KismetTextLibrary.Conv_StringToText` (`self.Antécédent`)))
    (if (`self.Vaccins`)
      (`TextRenderComponent.K2_SetText` (`self.Vaccin_txt`) (`KismetTextLibrary.Conv_StringToText` (`self.Vaccin a jour`)))
      (else
        (`TextRenderComponent.K2_SetText` (`self.Vaccin_txt`) (`KismetTextLibrary.Conv_StringToText` (`self.Vaccin pas a jour`)))))
    (`TextRenderComponent.K2_SetText` (`self.Addiction_txt`) (`KismetTextLibrary.Conv_StringToText` (`self.Addiction`)))
    (`TextRenderComponent.K2_SetText` (`self.Poids_txt`) (`KismetTextLibrary.Conv_IntToText` (`self.Poids`)))
    (`TextRenderComponent.K2_SetText` (`self.name_txt`) (`KismetTextLibrary.Conv_StringToText` (`self.Nom`)))
    (if (`self.Sexe`)
      (`TextRenderComponent.K2_SetText` _sex_txt (`KismetTextLibrary.Conv_StringToText` (`self.Homme`)))
      (else
        (`TextRenderComponent.K2_SetText` _sex_txt (`KismetTextLibrary.Conv_StringToText` (`self.Femme`)))))
    (`TextRenderComponent.K2_SetText` (`self.birth_txt`) (`KismetTextLibrary.Conv_IntToText` (`self.AnnéeNaissance`)))
    (`TextRenderComponent.K2_SetText` (`self.country_txt`) (`KismetTextLibrary.Conv_StringToText` (`self.Pays`)))
    (`TextRenderComponent.K2_SetText` (`self.tall_txt`) (`KismetTextLibrary.Conv_DoubleToText` (`self.Taille`) "HalfToEven"))
    (`TextRenderComponent.K2_SetText` (`self.permis_txt`) (`KismetTextLibrary.Conv_StringToText` (`self.Permis`)))
    (`TextRenderComponent.K2_SetText` (`self.study_txt`) (`KismetTextLibrary.Conv_StringToText` (`self.Etudes`)))
    (`self.SetActorHiddenInGame` false)
    (`ActorComponent.SetActive` _animchemise true false)
    (`PaperFlipbookComponent.SetLooping` _animchemise false)
    (bind (_direction _timestamp) (`Timeline|Timeline_0`)
      (:`Update`
        (`SceneComponent.K2_SetRelativeLocation` (`self.DefaultSceneRoot`) (`KismetMathLibrary.VLerp` (`SceneComponent.K2_GetComponentLocation` (`self.DefaultSceneRoot`)) (`self.EndLocation`) _timestamp) false false)
        (`KismetSystemLibrary.Delay` (`PaperFlipbookComponent.GetFlipbookLength` (`self.AnimChemise`)))
        (`SceneComponent.SetHiddenInGame` (`self.FeuilleVoyage`) false true)
        (`SceneComponent.SetHiddenInGame` (`self.Carte_identité`) false true)))))

(fn `InitArrays`
  (set `self.Antécédent` (`self.GetRandomArrayElement` (`self.Antécédents`)))
  (set `self.Addiction` (`self.GetRandomArrayElement` (`self.Addictions`)))
  (set `self.Permis` (`self.GetRandomArrayElement` (`self.ListePermis`)))
  (set `self.GroupeSanguin` (`self.GetRandomArrayElement` (`self.GroupesSanguins`)))
  (set `self.Etudes` (`self.GetRandomArrayElement` (`self.ListeEtudes`)))
  (set `self.Pays` (`self.GetRandomArrayElement` (`self.ListePays`)))
  (bind _output_get (set `self.Nom` (`self.GetRandomArrayElement` (`self.Noms`))))
  (bind _output_get_2 (set `self.Nom` (`KismetStringLibrary.Concat_StrStr` _output_get " ")))
  (set `self.Nom` (`KismetStringLibrary.Concat_StrStr` _output_get_2 (`self.GetRandomArrayElement` (`self.Prénoms`)))))

(fn `InitOthers`
  (set `self.PretImmo` (`KismetMathLibrary.RandomIntegerInRange` 1000 100000))
  (set `self.Revenu` (`KismetMathLibrary.RandomIntegerInRange` 300 6000))
  (set `self.ValeurImmo` (`KismetMathLibrary.RandomIntegerInRange` 150000 900000))
  (set `self.Poids` (`KismetMathLibrary.RandomIntegerInRange` 40 270))
  (set `self.AnnéeNaissance` (`KismetMathLibrary.RandomIntegerInRange` 1900 1955))
  (set `self.Taille` (`KismetMathLibrary.RandomFloatInRange` 1.4 2.0))
  (set `self.Sexe` (`KismetMathLibrary.RandomBool`))
  (set `self.Vaccins` (`KismetMathLibrary.RandomBool`)))

(fn `UserConstructionScript`
  (`SceneComponent.K2_SetWorldLocation` (`self.DefaultSceneRoot`) (30.0 -1100.0 710.0) false false)
  (bind _returnvalue (`AddComponent|NODE_AddPaperSpriteComponent-4` :`RelativeTransform` (`SceneComponent.GetRelativeTransform` (`self.cou_perso`))))
  (`PaperSpriteComponent.SetSprite` _returnvalue (`self.GetRandomArrayElement` (`self.Sprites_Cou`)))
  (bind _returnvalue_2 (`AddComponent|NODE_AddPaperSpriteComponent-5` :`RelativeTransform` (`SceneComponent.GetRelativeTransform` (`self.nez_perso`))))
  (`PaperSpriteComponent.SetSprite` _returnvalue_2 (`self.GetRandomArrayElement` (`self.Sprites_Nez`)))
  (bind _returnvalue_3 (`AddComponent|NODE_AddPaperSpriteComponent-9` :`RelativeTransform` (`SceneComponent.GetRelativeTransform` (`self.yeux_perso`))))
  (`PaperSpriteComponent.SetSprite` _returnvalue_3 (`self.GetRandomArrayElement` (`self.Sprites_Yeux`)))
  (bind _returnvalue_4 (`AddComponent|NODE_AddPaperSpriteComponent-6` :`RelativeTransform` (`SceneComponent.GetRelativeTransform` (`self.tete_perso`))))
  (`PaperSpriteComponent.SetSprite` _returnvalue_4 (`self.GetRandomArrayElement` (`self.Sprite_Tete`))))