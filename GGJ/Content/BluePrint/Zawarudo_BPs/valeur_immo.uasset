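; Blueprint that generates a random real estate value ("valeur immo") and derives a chance tier from it.
; On BeginPlay it rolls a random integer into Immo, then a cascade of threshold checks sets Chanceplus to a tier from 1 to 4, higher for pricier values.
; Both the value and the tier are printed to screen; nothing in this file consumes Chanceplus.
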(event `self.ReceiveBeginPlay`
  (bind _output_get (set `self.Immo` (`KismetMathLibrary.RandomIntegerInRange` 150000 900000)))
  (`KismetSystemLibrary.PrintString` (`KismetStringLibrary.Conv_IntToString` _output_get))
  (if (<= (`KismetMathLibrary.Conv_IntToDouble` (`self.Immo`)) 200000.0)
    (set `self.chanceplus` 1)
    (`KismetSystemLibrary.PrintString` "1")
    (elif (<= (`KismetMathLibrary.Conv_IntToDouble` (`self.Immo`)) 400000.0)
      (set `self.chanceplus` 2)
      (`KismetSystemLibrary.PrintString` "2")
      (elif (<= (`KismetMathLibrary.Conv_IntToDouble` (`self.Immo`)) 700000.0)
        (set `self.chanceplus` 3)
        (`KismetSystemLibrary.PrintString` "3")
        (elif (<= (`KismetMathLibrary.Conv_IntToDouble` (`self.Immo`)) 900000.0)
          (set `self.chanceplus` 4)
          (`KismetSystemLibrary.PrintString` "4"))))))

(fn `UserConstructionScript`)