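; Actor Blueprint that rolls a random PretImmo value (French for home loan, by its name) and prints a figure derived from it.
; On BeginPlay it picks a random multiple of 1000 up to 100000, then prints that value and a fixed constant divided by the value plus an offset.
; The result is only printed, and the overlap, tick and construction graphs are empty.
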(event `self.ReceiveBeginPlay`
  (bind _output_get (set `self.pret immo` (* (`KismetMathLibrary.RandomIntegerInRange` 1 100) 1000)))
  (`KismetSystemLibrary.PrintString` (`KismetStringLibrary.Conv_IntToString` _output_get))
  (`KismetSystemLibrary.PrintString` (`KismetStringLibrary.Conv_DoubleToString` (/ 123750.0 (+ (`KismetMathLibrary.Conv_IntToDouble` (`self.pret immo`)) 23750.0)))))

(fn `UserConstructionScript`)