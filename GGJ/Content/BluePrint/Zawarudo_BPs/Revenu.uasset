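; Revenu is an actor Blueprint that generates a random revenue value when play begins.
; BeginPlay rolls a random multiple of one hundred, stores it in Revenu and prints it.
; It also prints a linear remap of that value, which scales the revenue range onto roughly 3 to 7 without storing the result.
; Overlap, Tick and the construction script are empty.
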(event `self.ReceiveBeginPlay`
  (bind _output_get (set `self.revenu` (`KismetMathLibrary.FTrunc` (* (`KismetMathLibrary.RandomIntegerInRange` 3 60) 100.0))))
  (`KismetSystemLibrary.PrintString` (`KismetStringLibrary.Conv_IntToString` _output_get))
  (`KismetSystemLibrary.PrintString` (`KismetStringLibrary.Conv_DoubleToString` (+ (* (`KismetMathLibrary.Conv_IntToDouble` (`self.revenu`)) (/ 1.0 1425.0)) (/ 53.0 19.0)))))

(fn `UserConstructionScript`)